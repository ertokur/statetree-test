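; BP_Dummy is an example actor with health that reports its death to a StateTree.
; Health starts at MaxHealth on BeginPlay, and AnyDamage subtracts damage from it, clamped between zero and MaxHealth.
; When Health reaches zero, it sends a StateTree.Event.Dead event to its StateTree component, leaving the reaction to the tree.
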(event `self.ReceiveBeginPlay`
  (set `self.Health` (`self.MaxHealth`)))

(event `self.ReceiveAnyDamage`
  (params (Damage :type "Float (single-precision)") (DamageType :type "DamageType Object Reference") (InstigatedBy :type "Controller Object Reference") (DamageCauser :type "Actor Object Reference"))
  (set `self.Health` (`KismetMathLibrary.FClamp` (- (`self.Health`) Damage) 0.0 (`self.MaxHealth`)))
  (if (<= (`self.Health`) 0.0)
    (`StateTreeComponent.SendStateTreeEvent` (`self.StateTree`) (make `StateTreeEvent` (struct :`TagName` "StateTree.Event.Dead")))))

(fn `UserConstructionScript`)