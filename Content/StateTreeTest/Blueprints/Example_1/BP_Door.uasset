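; BP_Door is a sliding door actor in a StateTree example that tracks characters in a trigger sphere and can raise or lower its cube.
; Sphere overlaps maintain a list of characters inside and set CharacterEntered, clearing it only when the last one leaves.
; OpenDoor and CloseDoor set DoorOpen and play or reverse a timeline that lerps the cube's height.
; The overlap logic never calls these events itself.
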(event `self.Sphere.OnComponentBeginOverlap`
  (params (OverlappedComponent :type "PrimitiveComponent Object Reference") (OtherActor :type "Actor Object Reference") (OtherComp :type "PrimitiveComponent Object Reference") (OtherBodyIndex :type Integer) (bFromSweep :type Boolean) (SweepResult :type "HitResult Structure (by ref)"))
  (cast `Character` OtherActor)
  (`KismetArrayLibrary.Array_AddUnique` (`self.EnteredActors`) OtherActor)
  (set `self.bCharacterEntered` true))

(event `self.Sphere.OnComponentEndOverlap`
  (params (OverlappedComponent :type "PrimitiveComponent Object Reference") (OtherActor :type "Actor Object Reference") (OtherComp :type "PrimitiveComponent Object Reference") (OtherBodyIndex :type Integer))
  (cast `Character` OtherActor)
  (`KismetArrayLibrary.Array_RemoveItem` (`self.EnteredActors`) OtherActor)
  (if (`KismetArrayLibrary.Array_IsEmpty` (`self.EnteredActors`))
    (set `self.bCharacterEntered` false)))

(event `OpenDoor`
  (set `self.bDoorOpen` true)
  (bind (_direction _alpha) (`Timeline|DoorAnimation` :!label _label)
    (:`Update`
      (`SceneComponent.K2_SetRelativeLocation` (`self.Cube`) (`KismetMathLibrary.MakeVector` 0.0 0.0 (`KismetMathLibrary.Lerp` 0.0 200.0 _alpha)) false false))))

(event `CloseDoor`
  (set `self.bDoorOpen` false)
  (goto _label :!via `Reverse`))

(fn `UserConstructionScript`)