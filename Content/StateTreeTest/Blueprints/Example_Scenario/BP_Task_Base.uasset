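; BP_Task_Base is a task Blueprint in a StateTree example scenario, holding a task state and reacting to its StateTree's run status.
; SetTaskState stores the new TaskState, which Tick prints on screen every frame as a debug readout.
; When the StateTree run status changes to Succeeded, it prints a completion message, waits briefly, then stops the StateTree logic.
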(event `self.ReceiveBeginPlay`)

(event `self.ReceiveTick`
  (params (DeltaSeconds :type "Float (single-precision)"))
  (`KismetSystemLibrary.PrintString` (`|GetEnumeratorNameAsString` (`self.TaskState`)) true false (struct :`G` 0.66 :`B` 1.0 :`A` 1.0) 0.0))

(event `self.StateTree.OnStateTreeRunStatusChanged`
  (params (StateTreeRunStatus :type "EStateTreeRunStatus Enum" :default "Running"))
  (switch `EStateTreeRunStatus` StateTreeRunStatus
    (:`Succeeded`
      (`KismetSystemLibrary.PrintString` "Task completed")
      (`KismetSystemLibrary.Delay` 1.0)
      (`BrainComponent.StopLogic` (`self.StateTree`) ""))))

(fn `SetTaskState`
  (params (NewTaskState :type "/Game/StateTreeTest/Blueprints/Example_Scenario/E_TaskState Enum" :default "NewEnumerator0"))
  (set `self.TaskState` NewTaskState))

(fn `UserConstructionScript`)